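; Player character Blueprint that sets up the local HUD and handles inventory and camera-rotation input.
; BeginPlay adds crosshair and health indicator widgets for the locally controlled player; Tab lazily creates or reveals the inventory in UI-only mode with cursor.
; Holding Left Shift disables orient-to-movement and sets a CameraRotating flag.
; Health changes draw debug text at the actor, while disconnected trace and print experiments never run.
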(event OnHealthChanged(HealthComp)
  (params (HealthComp :type Health%20Component%20Object%20Reference) (Health :type Float%20%28single-precision%29) (HealthDelta :type Float%20%28single-precision%29) (DamageType :type Damage%20Type%20Object%20Reference) (InstigatedBy :type Controller%20Object%20Reference) (DamageCauser :type Actor%20Object%20Reference))
  (Rendering|Debug|DrawDebugString (Transformation|GetActorLocation) (Utilities|String|ToString(Float) Health) 0 "(R=1.000000,G=1.000000,B=1.000000,A=1.000000)"))

(event EventBeginPlay
  (bind _returnvalue (Game|GetPlayerController 0))
  (if (Pawn|IsLocallyControlled)
    (Utilities|FlowControl|Sequence
      (:then_0
        (bind _returnvalue_2 (UserInterface|CreateWidget "/Game/Blueprint/UI/WBP_Crosshair.WBP_Crosshair_C" _returnvalue))
        (UserInterface|Viewport|AddtoViewport _returnvalue_2 0))
      (:then_1
        (bind _returnvalue_3 (UserInterface|CreateWidget "/Game/Blueprint/UI/WBP_HealthIndicator.WBP_HealthIndicator_C" _returnvalue))
        (UserInterface|Viewport|AddtoViewport _returnvalue_3 0)))))

(event EventTick
  (params (DeltaSeconds :type Float%20%28single-precision%29)))

(event Input|KeyboardEvents|Tab
  (params (Key :type Key%20Structure :default "None"))
  (bind _returnvalue (Game|GetPlayerController 0))
  ;[1 1 1] Tab 입력시 WBP_Inventory가 nullptr이면 위젯을 생성 아니면 Hide상태를 VIsible로 바꾸고 UI만 입력가능하게 바꿈
  (:Pressed
    (Utilities|IsValid (Variables|Default|GetInventory)
      (:Is%20Valid
        (Widget|SetVisibility (Variables|Default|GetInventory) "Visible"))
      (:Is%20Not%20Valid
        (bind _returnvalue_2 (UserInterface|CreateWidget "/Game/Blueprint/UI/WBP_Inventory.WBP_Inventory_C" (Game|GetPlayerController 0)))
        (UserInterface|Viewport|AddtoViewport _returnvalue_2 0)
        (bind _output_get (Variables|Default|SetInventory _returnvalue_2))))
    (Input|SetInputModeUIOnly _returnvalue (Variables|Default|GetInventory) "DoNotLock")
    (Variables|/Script/Engine.PlayerController|SetbShowMouseCursor _returnvalue true)
    (Widget|SetFocus _output_get)))

(event Input|KeyboardEvents|LeftShift
  (params (Key :type Key%20Structure :default "None"))
  (bind _charactermovement (Variables|Character|GetCharacterMovement))
  (:Pressed
    (Variables|/Script/Engine.CharacterMovementComponent|SetbOrientRotationToMovement _charactermovement false)
    (Variables|Default|SetbCameraRotating true))
  (:Released
    (Variables|/Script/Engine.CharacterMovementComponent|SetbOrientRotationToMovement _charactermovement true)
    (Variables|Default|SetbCameraRotating false)))

(fn ConstructionScript)